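; BP_SpeciesLookupDemo is a demo actor that looks up a Pokémon species in a data table and prints its data for inspection.
; On BeginPlay it fetches the RowToQuery row from SpeciesTable and prints its types, base stats and catch rate.
; It then loops over the row's move list, printing each move with the level it is learnt at.
; A missing row prints a not-found message instead.
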(event EventBeginPlay
  (bind _rowtoquery (Variables|Default|GetRowToQuery))
  (bind _returnvalue (Utilities|String|ToString(Name) _rowtoquery))
  (bind _returnvalue_2 (Utilities|GetDataTableRow (Variables|Default|GetSpeciesTable) _rowtoquery)
    (:then
      (Development|PrintString (Utilities|String|Append "Species: " _returnvalue))
      (Development|PrintString (Utilities|String|Append "Type 1: " (.Type1 (Utilities|Struct|BreakS_PokemonSpeciesData _returnvalue_2))))
      (Development|PrintString (Utilities|String|Append "Type 2: " (.Type2 (Utilities|Struct|BreakS_PokemonSpeciesData _returnvalue_2))))
      (Development|PrintString (Utilities|String|Append "HP: " (Utilities|String|ToString(Integer) (.HP (Utilities|Struct|BreakS_PokemonStats (.BaseStats (Utilities|Struct|BreakS_PokemonSpeciesData _returnvalue_2)))))))
      (Development|PrintString (Utilities|String|Append "Attack: " (Utilities|String|ToString(Integer) (.Attack (Utilities|Struct|BreakS_PokemonStats (.BaseStats (Utilities|Struct|BreakS_PokemonSpeciesData _returnvalue_2)))))))
      (Development|PrintString (Utilities|String|Append "Defence: " (Utilities|String|ToString(Integer) (.Defence (Utilities|Struct|BreakS_PokemonStats (.BaseStats (Utilities|Struct|BreakS_PokemonSpeciesData _returnvalue_2)))))))
      (Development|PrintString (Utilities|String|Append "Sp. Attack: " (Utilities|String|ToString(Integer) (.SpAttack (Utilities|Struct|BreakS_PokemonStats (.BaseStats (Utilities|Struct|BreakS_PokemonSpeciesData _returnvalue_2)))))))
      (Development|PrintString (Utilities|String|Append "Sp. Defence: " (Utilities|String|ToString(Integer) (.SpDefence (Utilities|Struct|BreakS_PokemonStats (.BaseStats (Utilities|Struct|BreakS_PokemonSpeciesData _returnvalue_2)))))))
      (Development|PrintString (Utilities|String|Append "Speed: " (Utilities|String|ToString(Integer) (.Speed (Utilities|Struct|BreakS_PokemonStats (.BaseStats (Utilities|Struct|BreakS_PokemonSpeciesData _returnvalue_2)))))))
      (Development|PrintString (Utilities|String|Append "Base Catch Rate: " (Utilities|String|ToString(Integer) (.BaseCatchRate (Utilities|Struct|BreakS_PokemonSpeciesData _returnvalue_2)))))
      (Development|PrintString "--- Move List ---")
      (for _array_element (.MoveList (Utilities|Struct|BreakS_PokemonSpeciesData _returnvalue_2))
        (Development|PrintString (Utilities|String|Append "Move: " (Utilities|String|ToString(Name) (.MoveName (Utilities|Struct|BreakS_TMMove _array_element)))))
        (Development|PrintString (Utilities|String|Append "  Learned at Level: " (Utilities|String|ToString(Integer) (.LevelLearnt (Utilities|Struct|BreakS_TMMove _array_element)))))))
    (:RowNotFound
      (Development|PrintString (Utilities|String|Append "Row not found in Species DataTable: " _returnvalue)))))

(event Collision|EventActorBeginOverlap
  (params (OtherActor :type Actor%20Object%20Reference)))

(event EventTick
  (params (DeltaSeconds :type Float%20%28single-precision%29)))

(fn ConstructionScript)