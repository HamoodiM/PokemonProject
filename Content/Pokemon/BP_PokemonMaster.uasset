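; Base Pokémon character Blueprint that configures its stats, identity and sprite from a species data table row.
; InitializeFromSpecies runs from both the construction script and BeginPlay, filling PokemonStats and PokemonData and setting the Paper2D flipbook, or printing an error if the row is missing.
; A separate UpdateWalkSpeed function sets the movement component's max walk speed.
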(event EventBeginPlay
  (CallFunction|InitializefromSpecies))

(event Collision|EventActorBeginOverlap
  (params (OtherActor :type Actor%20Object%20Reference)))

(event EventTick
  (params (DeltaSeconds :type Float%20%28single-precision%29)))

(fn ConstructionScript
  (CallFunction|InitializefromSpecies))

(fn InitializefromSpecies
  (bind _speciesrow (Variables|Default|GetSpeciesRow))
  (bind _returnvalue (Utilities|GetDataTableRow (Variables|Default|GetSpeciesTable) _speciesrow)
    (:then
      (Variables|Default|SetPokemonStats (.BaseStats (Utilities|Struct|BreakS_PokemonSpeciesData _returnvalue)))
      (Variables|Default|SetPokemonData (Utilities|Struct|MakeS_Pokemon (.PokedexNumber (Utilities|Struct|BreakS_PokemonSpeciesData _returnvalue)) _speciesrow (Utilities|Text|ToText(Name) _speciesrow) (Utilities|String|StringToName (.Type1 (Utilities|Struct|BreakS_PokemonSpeciesData _returnvalue))) (Utilities|String|StringToName (.Type2 (Utilities|Struct|BreakS_PokemonSpeciesData _returnvalue))) "" "" "" (.Sprite (Utilities|Struct|BreakS_PokemonSpeciesData _returnvalue)) "" "" "" "" 1 100))
      (bind _aspaper_flipbook_component (Utilities|Casting|CastToPaperFlipbookComponent (Actor|GetComponentbyClass self "/Script/Paper2D.PaperFlipbookComponent")))
      (Sprite|SetFlipbook _aspaper_flipbook_component (.Sprite (Utilities|Struct|BreakS_PokemonSpeciesData _returnvalue))))
    (:RowNotFound
      (Development|PrintString (Utilities|String|Append "Species row not found: " (Utilities|String|ToString(Name) _speciesrow))))))

(fn UpdateWalkSpeed
  (params (NewWalkSpeed :type Float%20%28double-precision%29))
  (Variables|/Script/Engine.CharacterMovementComponent|SetMaxWalkSpeed (Variables|Character|GetCharacterMovement) NewWalkSpeed))