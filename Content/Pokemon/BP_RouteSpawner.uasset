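; Spawns random wild Pokémon in a route volume as the player walks through it, like step-based encounters.
; Tick accumulates player distance inside the volume, rolling a spawn chance each step interval while live spawns stay below a cap.
; Each spawn tries up to ten random points in the volume's bounds at center height, spaced from player and other spawns, then initializes a BP_PokemonMaster with a random species.
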(event EventBeginPlay
  (bind _routevolume (Variables|Default|GetRouteVolume))
  (bind (_origin _boxextent) (Collision|GetActorBounds _routevolume false false))
  (Variables|Default|SetRouteOrigin _origin)
  (Variables|Default|SetRouteExtent _boxextent)
  (Variables|Default|SetPlayerRef (Game|GetPlayerCharacter 0)))

(event Collision|EventActorBeginOverlap
  (params (OtherActor :type Actor%20Object%20Reference)))

(event EventTick
  (params (DeltaSeconds :type Float%20%28single-precision%29))
  (bind _playerref (Variables|Default|GetPlayerRef))
  (bind _stepdistance (Variables|Default|GetStepDistance))
  (bind _returnvalue (Transformation|GetActorLocation _playerref))
  (if (Collision|IsOverlappingActor (Variables|Default|GetRouteVolume) _playerref :!class /Script/Engine.Actor)
    (if (Variables|Default|GetPlayerInRoute)
      (Variables|Default|SetAccumulatedDistance (+ (Variables|Default|GetAccumulatedDistance) (Math|Vector|Distance(Vector) _returnvalue (Variables|Default|GetLastPlayerLocation))))
      (Variables|Default|SetLastPlayerLocation _returnvalue)
      (while (>= (Variables|Default|GetAccumulatedDistance) _stepdistance)
        (Variables|Default|SetAccumulatedDistance (- (Variables|Default|GetAccumulatedDistance) _stepdistance))
        (CallFunction|RollSpawnChance))
      (else
        (Variables|Default|SetPlayerInRoute true)
        (Variables|Default|SetAccumulatedDistance 0.0)
        (Variables|Default|SetLastPlayerLocation (Transformation|GetActorLocation _playerref))))
    (else
      (Variables|Default|SetPlayerInRoute false)
      (Variables|Default|SetAccumulatedDistance 0.0))))

(fn ConstructionScript)

(fn RollSpawnChance
  (bind _array (Utilities|Array|MakeArray 0))
  (for _array_element (Variables|Default|GetWildPokemonList)
    (Utilities|IsValid _array_element
      (:Is%20Valid
        (Utilities|Array|Add _array _array_element))))
  (Variables|Default|SetWildPokemonList _array)
  (if (< (Utilities|Array|Length (Variables|Default|GetWildPokemonList)) (Variables|Default|GetMaxConcurrentWild))
    (if (<= (Math|Random|RandomFloatinRange 0.0 1.0) (Variables|Default|GetSpawnChancePerStep))
      (CallFunction|TrySpawnWildPokemon))))

(fn TrySpawnWildPokemon
  (bind _routeextent (Variables|Default|GetRouteExtent))
  (bind _routeorigin (Variables|Default|GetRouteOrigin))
  (bind _speciesrows (Variables|Default|GetSpeciesRows))
  (Variables|Default|SetTempCandidateValid false)
  (for _index (range 0 9)
    (if (not (Variables|Default|GetTempCandidateValid))
      (Variables|Default|SetTempCandidateLoc (Math|Vector|MakeVector (+ (.X (Math|Vector|BreakVector _routeorigin)) (Math|Random|RandomFloatinRange (- 0.0 (.X (Math|Vector|BreakVector _routeextent))) (.X (Math|Vector|BreakVector _routeextent)))) (+ (.Y (Math|Vector|BreakVector _routeorigin)) (Math|Random|RandomFloatinRange (- 0.0 (.Y (Math|Vector|BreakVector _routeextent))) (.Y (Math|Vector|BreakVector _routeextent)))) (.Z (Math|Vector|BreakVector _routeorigin))))
      (if (>= (Math|Vector|Distance(Vector) (Variables|Default|GetTempCandidateLoc) (Transformation|GetActorLocation (Variables|Default|GetPlayerRef))) (Variables|Default|GetMinDistanceFromPlayer))
        (bind _returnvalue (CallFunction|IsSpawnLocationValid (Variables|Default|GetTempCandidateLoc)))
        (if _returnvalue
          (Variables|Default|SetTempCandidateValid true)))))
  (if (Variables|Default|GetTempCandidateValid)
    (bind _returnvalue_2 (Game|SpawnActorfromClass "/Game/Pokemon/BP_PokemonMaster.BP_PokemonMaster_C" (Math|Transform|MakeTransform (Variables|Default|GetTempCandidateLoc)) "AlwaysSpawn" "MultiplyWithRoot" 0 0))
    (Variables|/Game/Pokemon/BP_PokemonMaster.BP_PokemonMaster_C|SetSpeciesRow _returnvalue_2 (Utilities|Array|Get(acopy) _speciesrows (Math|Random|RandomIntegerinRange 0 (- (Utilities|Array|Length _speciesrows) (Class|KismetSystemLibrary|MakeLiteralInteger 1)))))
    (Default|InitializefromSpecies _returnvalue_2)
    (Utilities|Array|Add (Variables|Default|GetWildPokemonList) _returnvalue_2)))

(fn IsSpawnLocationValid
  (params (Candidate :type Vector))
  (for _array_element (Variables|Default|GetWildPokemonList)
    (Utilities|IsValid _array_element
      (:Is%20Valid
        (if (< (Math|Vector|Distance(Vector) Candidate (Transformation|GetActorLocation _array_element)) (Variables|Default|GetMinDistanceBetweenWild))
          (return false)))))
  (return true))