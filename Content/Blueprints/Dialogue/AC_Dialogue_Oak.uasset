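; Dialogue component for Prof. Oak that runs the starter Pokemon choice, or a short farewell once StarterChosen is set on the game instance.
; Dialogue replays from the top on each progress step, with AddDialogue returning recorded answers from the DialogueProgress map or updating W_Dialogue.
; Without a starter, it opens WBP_StarterSelect; a selection creates a level 5 Pokemon, adds it to the party, sets the flag and closes the conversation.
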(fn OpenConversation
  (Utilities|IsValid (Variables|Default|GetDialogueWidget)
    (:Is%20Not%20Valid
      (bind _returnvalue (UserInterface|CreateWidget "/Game/Blueprints/UI/W_Dialogue.W_Dialogue_C" 0 self))
      (bind _output_get (Variables|Default|SetDialogueWidget _returnvalue))
      (UserInterface|Viewport|AddtoViewport _output_get 0)
      (CallFunction|ProgressDialogue))))

(fn CloseConversation
  (Widget|RemovefromParent (Variables|Default|GetDialogueWidget))
  (Class|BPIInteractable|ConversationClosed(Message) (Components|GetOwner))
  (Variables|Default|SetDialogueWidget 0))

(fn ProgressDialogue
  (Variables|Default|SetDialogueIndex -1)
  (CallFunction|Dialogue))

(fn Dialogue
  (bind _asbp_pokemon_game_instance (Utilities|Casting|CastToBP_PokemonGameInstance (Game|GetGameInstance)))
  (if (Variables|/Game/Blueprints/BP_PokemonGameInstance.BP_PokemonGameInstance_C|GetbStarterChosen _asbp_pokemon_game_instance)
    (CallFunction|AddDialogue "Prof. Oak" "Take good care of your Pokemon partner!" 0)
    (CallFunction|CloseConversation)
    (else
      (CallFunction|AddDialogue "Prof. Oak" "Ah, welcome to my lab! Every young trainer needs a Pokemon partner. Go on, pick the one that speaks to you." 0)
      (CallFunction|OpenStarterSelectWidget))))

(fn AddDialogue
  (params (Speaker :type Text) (Dialogue :type Text) (OptionsText :type Array%20of%20Texts))
  (bind _dialogueprogress (Variables|Default|GetDialogueProgress))
  (bind _dialogueindex (Variables|Default|GetDialogueIndex))
  (bind (_value _returnvalue) (Utilities|Map|Find _dialogueprogress _dialogueindex))
  (Math|Integer|IncrementInt (Variables|Default|GetDialogueIndex)
    (:%20%20
      (if _returnvalue
        (return "NewEnumerator0" _value)
        (else
          (Default|UpdateText (Variables|Default|GetDialogueWidget) (Utilities|String|ToString(Text) Dialogue) (Variables|Default|GetDialogueIndex) Speaker Dialogue OptionsText)
          (return "NewEnumerator1" 0))))))

(fn UpdateSelectedOption
  (params (ProgressIndex :type Integer%20%28by%20ref%29) (OptionIndex :type Integer%20%28by%20ref%29))
  (Utilities|Map|Add (Variables|Default|GetDialogueProgress) ProgressIndex OptionIndex)
  (CallFunction|ProgressDialogue))

(fn ClearDialogueProgress
  (Utilities|Map|Clear (Variables|Default|GetDialogueProgress)))

(fn RemoveDialogueProgress
  (params (ProgressSteps :type Integer))
  (for _index (range 0 ProgressSteps)
    (Utilities|Map|Remove (Variables|Default|GetDialogueProgress) (- (Variables|Default|GetDialogueIndex) _index))))

(fn SetDialogeTreeIndex
  (params (DialogueTreeIndex :type Integer))
  (Variables|Default|SetDialogueTreeIndex DialogueTreeIndex)
  (CallFunction|ClearDialogueProgress))

(fn GetDialogueTreeIndex
  (return (Variables|Default|GetDialogueTreeIndex)))

(fn OpenStarterSelectWidget
  (bind _returnvalue (UserInterface|CreateWidget "/Game/Blueprints/UI/WBP_StarterSelect.WBP_StarterSelect_C"))
  (bind _output_get (Variables|Default|SetActiveStarterWidget _returnvalue))
  (EventDispatchers|BindEventtoOnStarterSelected _output_get (EventDispatchers|CreateEvent self :!event HandleStarterSelected))
  (EventDispatchers|BindEventtoOnMenuClosed _output_get (EventDispatchers|CreateEvent self :!event HandleStarterMenuClosed))
  (UserInterface|Viewport|AddtoViewport _output_get 200))

(fn HandleStarterSelected
  (params (SpeciesRow :type Name))
  (bind _self self)
  (Widget|RemovefromParent (Variables|Default|GetActiveStarterWidget))
  (bind (_found _pokemon _stats _moves) (CallFunction|MakePokemonfromSpecies SpeciesRow 5 "/Game/Pokemon/DT_PokemonSpecies.DT_PokemonSpecies"))
  (if _found
    (bind _asbp_pokemon_game_instance (Utilities|Casting|CastToBP_PokemonGameInstance (Game|GetGameInstance)))
    (Default|AddtoParty _asbp_pokemon_game_instance (Utilities|Struct|MakeS_PartyMember _pokemon _stats _moves))
    (Variables|/Game/Blueprints/BP_PokemonGameInstance.BP_PokemonGameInstance_C|SetbStarterChosen _asbp_pokemon_game_instance true)
    (CallFunction|AddDialogue _self "Prof. Oak" "Take good care of your new partner! I know the two of you will do great things together." 0)
    (CallFunction|CloseConversation _self)))

(fn HandleStarterMenuClosed
  (Widget|RemovefromParent (Variables|Default|GetActiveStarterWidget)))