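; Dialogue component for Pink, the NPC Professor Eleena, who offers a Pokémon starter choice of Charmander, Squirtle or Bulbasaur.
; The Dialogue override calls its parent, then branches on the tree index and each AddDialogue state.
; Picking a starter only shows confirmation and advances the index, so later talks refuse seconds.
; Asking for more information describes the types, then rolls back dialogue progress and closes the conversation.
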(fn Dialogue
  (|CallParentFunction)
  (switch int (Variables|Default|GetDialogueTreeIndex)
    (:Default
      (bind _state (CallFunction|AddDialogue "Pink" "Hey! You've already gotten a starter, no seconds mister!" (Utilities|Array|MakeArray "Continue") :!label _label))
      (switch Utilities|FlowControl|Switch|SwitchonEnum_DialogueState _state
        (:NewEnumerator0
          (CallFunction|ClearDialogueProgress)
          (CallFunction|CloseConversation))))
    (:0
      (bind (_state_2 _option_index) (CallFunction|AddDialogue "Pink" "Hi! I'm Eleena, the Booey and Beengo  region's Professor! What starter are you interested in? " (Utilities|Array|MakeArray "Charmander" "Squirtle" "Bulbasaur" "Can you please tell me more about these options?")))
      (switch Utilities|FlowControl|Switch|SwitchonEnum_DialogueState _state_2
        (:NewEnumerator0
          (switch int _option_index
            (:0
              (bind _state_3 (CallFunction|AddDialogue "Pink" "Your starter is now Charmander!" (Utilities|Array|MakeArray "Continue")))
              (switch Utilities|FlowControl|Switch|SwitchonEnum_DialogueState _state_3
                (:NewEnumerator0
                  (CallFunction|SetDialogeTreeIndex 1)
                  (CallFunction|CloseConversation))))
            (:1
              (bind _state_4 (CallFunction|AddDialogue "Pink" "Your Starter is now Squirtle!" (Utilities|Array|MakeArray "Continue")))
              (switch Utilities|FlowControl|Switch|SwitchonEnum_DialogueState _state_4
                (:NewEnumerator0
                  (CallFunction|SetDialogeTreeIndex 1)
                  (CallFunction|CloseConversation))))
            (:2
              (bind _state_5 (CallFunction|AddDialogue "Pink" "Your starter is now Bulbasaur!" (Utilities|Array|MakeArray "Continue")))
              (switch Utilities|FlowControl|Switch|SwitchonEnum_DialogueState _state_5
                (:NewEnumerator0
                  (CallFunction|SetDialogeTreeIndex 1)
                  (CallFunction|CloseConversation))))
            (:3
              (bind _state_6 (CallFunction|AddDialogue "Pink" "Charmander is the ambitious fire type, Squirtle is the swagger water type, and Bulbasaur is the calm grass type! Come back when you have decided" (Utilities|Array|MakeArray "Continue")))
              (switch Utilities|FlowControl|Switch|SwitchonEnum_DialogueState _state_6
                (:NewEnumerator0
                  (CallFunction|RemoveDialogueProgress 2)
                  (CallFunction|CloseConversation))))))))
    (:1
      (goto _label))))