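; Poke Mart shopkeeper dialogue component that sells Poke Balls, Potions and Antidotes for money held in BP_PokemonGameInstance.
; OpenConversation creates W_Dialogue, and Dialogue branches on the chosen option to buy or close, looping after each result.
; AddDialogue shows the first unanswered step and passes through choices recorded in DialogueProgress.
; Each UpdateSelectedOption replays the tree from the start, re-running purchase side effects along the way.
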(fn OpenConversation
  (Utilities|IsValid (Variables|Default|GetDialogueWidget)
    (:Is%20Not%20Valid
      (bind _returnvalue (UserInterface|CreateWidget "/Game/Blueprints/UI/W_Dialogue.W_Dialogue_C" 0 self))
      (bind _output_get (Variables|Default|SetDialogueWidget _returnvalue))
      (UserInterface|Viewport|AddtoViewport _output_get 0)
      (CallFunction|ProgressDialogue))))

(fn CloseConversation
  (Widget|RemovefromParent (Variables|Default|GetDialogueWidget))
  (Class|BPIInteractable|ConversationClosed(Message) (Components|GetOwner))
  (Variables|Default|SetDialogueWidget 0))

(fn ProgressDialogue
  (Variables|Default|SetDialogueIndex -1)
  (CallFunction|Dialogue))

(fn Dialogue
  (bind _returnvalue (Game|GetGameInstance))
  (switch int (Variables|Default|GetDialogueTreeIndex)
    (:0
      (bind (_state _option_index) (CallFunction|AddDialogue "Shopkeeper" "Welcome to the Poke Mart! What would you like to buy?" 0))
      (switch Utilities|FlowControl|Switch|SwitchonEnum_DialogueState _state
        (:NewEnumerator0
          (switch int _option_index
            (:0
              (bind _asbp_pokemon_game_instance (Utilities|Casting|CastToBP_PokemonGameInstance _returnvalue)
                (:then
                  (if (>= (Variables|/Game/Blueprints/BP_PokemonGameInstance.BP_PokemonGameInstance_C|GetMoney _asbp_pokemon_game_instance) (Class|KismetSystemLibrary|MakeLiteralInteger 200))
                    (Default|RemoveMoney _asbp_pokemon_game_instance 200)
                    (Default|AddItem _asbp_pokemon_game_instance "PokeBall" 1)
                    (bind _state_2 (CallFunction|AddDialogue "Shopkeeper" "Here you go!" 0))
                    (switch Utilities|FlowControl|Switch|SwitchonEnum_DialogueState _state_2
                      (:NewEnumerator0
                        (CallFunction|Dialogue)))
                    (else
                      (bind _state_3 (CallFunction|AddDialogue "Shopkeeper" "You don't have enough money!" 0))
                      (switch Utilities|FlowControl|Switch|SwitchonEnum_DialogueState _state_3
                        (:NewEnumerator0
                          (CallFunction|Dialogue))))))
                (:CastFailed
                  (Development|PrintString "CastFailed"))))
            (:1
              (bind _asbp_pokemon_game_instance_2 (Utilities|Casting|CastToBP_PokemonGameInstance _returnvalue)
                (:then
                  (if (>= (Variables|/Game/Blueprints/BP_PokemonGameInstance.BP_PokemonGameInstance_C|GetMoney _asbp_pokemon_game_instance_2) (Class|KismetSystemLibrary|MakeLiteralInteger 300))
                    (Default|RemoveMoney _asbp_pokemon_game_instance_2 300)
                    (Default|AddItem _asbp_pokemon_game_instance_2 "Potion" 1)
                    (bind _state_4 (CallFunction|AddDialogue "Shopkeeper" "Here you go!" 0))
                    (switch Utilities|FlowControl|Switch|SwitchonEnum_DialogueState _state_4
                      (:NewEnumerator0
                        (CallFunction|Dialogue)))
                    (else
                      (bind _state_5 (CallFunction|AddDialogue "Shopkeeper" "You don't have enough money!" 0))
                      (switch Utilities|FlowControl|Switch|SwitchonEnum_DialogueState _state_5
                        (:NewEnumerator0
                          (CallFunction|Dialogue))))))
                (:CastFailed
                  (Development|PrintString "CastFailed"))))
            (:2
              (bind _asbp_pokemon_game_instance_3 (Utilities|Casting|CastToBP_PokemonGameInstance _returnvalue)
                (:then
                  (if (>= (Variables|/Game/Blueprints/BP_PokemonGameInstance.BP_PokemonGameInstance_C|GetMoney _asbp_pokemon_game_instance_3) (Class|KismetSystemLibrary|MakeLiteralInteger 150))
                    (Default|RemoveMoney _asbp_pokemon_game_instance_3 150)
                    (Default|AddItem _asbp_pokemon_game_instance_3 "Antidote" 1)
                    (bind _state_6 (CallFunction|AddDialogue "Shopkeeper" "Here you go!" 0))
                    (switch Utilities|FlowControl|Switch|SwitchonEnum_DialogueState _state_6
                      (:NewEnumerator0
                        (CallFunction|Dialogue)))
                    (else
                      (bind _state_7 (CallFunction|AddDialogue "Shopkeeper" "You don't have enough money!" 0))
                      (switch Utilities|FlowControl|Switch|SwitchonEnum_DialogueState _state_7
                        (:NewEnumerator0
                          (CallFunction|Dialogue))))))
                (:CastFailed
                  (Development|PrintString "Antidote cast to BP_PokemonGameInstance failed"))))
            (:3
              (CallFunction|CloseConversation))))))))

(fn AddDialogue
  (params (Speaker :type Text) (Dialogue :type Text) (OptionsText :type Array%20of%20Texts))
  (bind _dialogueprogress (Variables|Default|GetDialogueProgress))
  (bind _dialogueindex (Variables|Default|GetDialogueIndex))
  (bind (_value _returnvalue) (Utilities|Map|Find _dialogueprogress _dialogueindex))
  (Math|Integer|IncrementInt (Variables|Default|GetDialogueIndex)
    (:%20%20
      (if _returnvalue
        (return "NewEnumerator0" _value)
        (else
          (Default|UpdateText (Variables|Default|GetDialogueWidget) (Utilities|String|ToString(Text) Dialogue) (Variables|Default|GetDialogueIndex) Speaker Dialogue OptionsText)
          (return "NewEnumerator1" 0))))))

(fn UpdateSelectedOption
  (params (ProgressIndex :type Integer%20%28by%20ref%29) (OptionIndex :type Integer%20%28by%20ref%29))
  (Utilities|Map|Add (Variables|Default|GetDialogueProgress) ProgressIndex OptionIndex)
  (CallFunction|ProgressDialogue))

(fn ClearDialogueProgress
  (Utilities|Map|Clear (Variables|Default|GetDialogueProgress)))

(fn RemoveDialogueProgress
  (params (ProgressSteps :type Integer))
  (for _index (range 0 ProgressSteps)
    (Utilities|Map|Remove (Variables|Default|GetDialogueProgress) (- (Variables|Default|GetDialogueIndex) _index))))

(fn SetDialogeTreeIndex
  (params (DialogueTreeIndex :type Integer))
  (Variables|Default|SetDialogueTreeIndex DialogueTreeIndex)
  (CallFunction|ClearDialogueProgress))

(fn GetDialogueTreeIndex
  (return (Variables|Default|GetDialogueTreeIndex)))