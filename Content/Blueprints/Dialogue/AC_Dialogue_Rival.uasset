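; Dialogue component for the rival NPC that gates and launches the starter battle against the player.
; The first tree branch turns away a player with an empty party; otherwise it picks the starter that beats the lead Pokémon's primary type.
; That pick becomes the rival's single low-level party before the trainer battle starts with the interacting instigator.
; The second tree branch plays a post-defeat line and closes the conversation.
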(event EventDialogue
  (bind _asnpc_rival (Utilities|Casting|CastToNPC_Rival (Components|GetOwner)))
  (switch int (Variables|Default|GetDialogueTreeIndex)
    (:0
      (bind _asbp_pokemon_game_instance (Utilities|Casting|CastToBP_PokemonGameInstance (Game|GetGameInstance)))
      (if (== (Utilities|Array|Length (Variables|/Game/Blueprints/BP_PokemonGameInstance.BP_PokemonGameInstance_C|GetParty _asbp_pokemon_game_instance)) (Class|KismetSystemLibrary|MakeLiteralInteger))
        (bind _state (CallFunction|AddDialogue (Variables|/Game/Blueprints/Trainers/NPC_Trainer.NPC_Trainer_C|GetCharacterName _asnpc_rival) (Utilities|Text|ToText(String) "Hey! Go see the Professor first, you can't battle me without a Pokémon!") (Utilities|Array|MakeArray (Utilities|Text|ToText(String) "Continue"))))
        (switch Utilities|FlowControl|Switch|SwitchonEnum_DialogueState _state
          (:NewEnumerator0
            (CallFunction|CloseConversation)))
        (else
          (bind _returnvalue (CallFunction|GetTypeAdvantageStarter (.Type1 (Utilities|Struct|BreakS_Pokemon (.Pokemon (Utilities|Struct|BreakS_PartyMember (Utilities|Array|Get(acopy) (Variables|/Game/Blueprints/BP_PokemonGameInstance.BP_PokemonGameInstance_C|GetParty _asbp_pokemon_game_instance))))))))
          (bind _state_2 (CallFunction|AddDialogue (Variables|/Game/Blueprints/Trainers/NPC_Trainer.NPC_Trainer_C|GetCharacterName _asnpc_rival) (Utilities|Text|ToText(String) "So that's your partner, huh? I'll pick the one that beats it!") (Utilities|Array|MakeArray (Utilities|Text|ToText(String) "Continue"))))
          (switch Utilities|FlowControl|Switch|SwitchonEnum_DialogueState _state_2
            (:NewEnumerator0
              (Variables|/Game/Blueprints/Trainers/NPC_Trainer.NPC_Trainer_C|SetTrainerPartyRows _asnpc_rival (Utilities|Array|MakeArray _returnvalue))
              (Variables|/Game/Blueprints/Trainers/NPC_Trainer.NPC_Trainer_C|SetTrainerPartyLevels _asnpc_rival (Utilities|Array|MakeArray (Class|KismetSystemLibrary|MakeLiteralInteger 5)))
              (CallFunction|CloseConversation)
              (Default|StartTrainerBattle _asnpc_rival (Variables|/Game/Blueprints/Trainers/NPC_Trainer.NPC_Trainer_C|GetInteractInstigator _asnpc_rival)))))))
    (:1
      (bind _state_3 (CallFunction|AddDialogue (Variables|/Game/Blueprints/Trainers/NPC_Trainer.NPC_Trainer_C|GetCharacterName _asnpc_rival) (Utilities|Text|ToText(String) "You already beat me, huh? I'll get stronger and we'll battle again someday!") (Utilities|Array|MakeArray (Utilities|Text|ToText(String) "Continue"))))
      (switch Utilities|FlowControl|Switch|SwitchonEnum_DialogueState _state_3
        (:NewEnumerator0
          (CallFunction|CloseConversation))))))