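; NPC_Rival is the rival trainer NPC that the player can talk to in a Pokémon game.
; An interactable-state event toggles a name text's visibility, and interacting stores the instigator, opens the rival dialogue component's conversation and notifies that instigator when it closes.
; BeginPlay copies the rival's name from the game instance, but the name label text is set only in the construction script.
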(event EventConversationClosed
  (Class|BPIInteractable|ConversationClosed(Message) (Variables|Default|GetInteractInstigator)))

(event EventInteract
  (params (Instigator :type Actor%20Object%20Reference))
  (Variables|Default|SetInteractInstigator Instigator)
  (Default|OpenConversation (Variables|Default|GetAC_Dialogue_Rival)))

(event EventBeginPlay
  (bind _asbp_pokemon_game_instance (Utilities|Casting|CastToBP_PokemonGameInstance (Game|GetGameInstance)))
  (Variables|Default|SetCharacterName (Variables|/Game/Blueprints/BP_PokemonGameInstance.BP_PokemonGameInstance_C|GetRivalName _asbp_pokemon_game_instance)))

(event EventSetInteractableState
  (params (bCanShowInteract? :type Boolean))
  (if bCanShowInteract?
    (Rendering|SetVisibility (Variables|Default|GetTxt_CharacterName_0) true false)
    (else
      (Rendering|SetVisibility (Variables|Default|GetTxt_CharacterName_0) false false))))

(fn ConstructionScript
  (Rendering|Components|TextRender|SetText (Variables|Default|GetTxt_CharacterName) (Variables|Default|GetCharacterName)))