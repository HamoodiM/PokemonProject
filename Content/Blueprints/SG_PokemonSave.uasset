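; SaveGame object that holds the player's progress in a Pokemon-style game.
; It stores the starter choice, the party, the player's location and rotation, and a dialogue tree index named Pink.
; Populate writes all of these fields in one call, and GetData returns them together.
; It only carries data; the file contains no save or load calls.
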(fn Populate
  (params (bStarterChosen :type Boolean) (Party :type Array%20of%20S%20Party%20Member%20Structures) (PlayerLocation :type Vector) (PlayerRotation :type Rotator) (DialogueTreeIndexPink :type Integer))
  (Variables|Default|SetbStarterChosen bStarterChosen)
  (Variables|Default|SetParty Party)
  (Variables|Default|SetPlayerLocation PlayerLocation)
  (Variables|Default|SetPlayerRotation PlayerRotation)
  (Variables|Default|SetDialogueTreeIndex_Pink DialogueTreeIndexPink))

(fn GetData
  (return (Variables|Default|GetbStarterChosen) (Variables|Default|GetParty) (Variables|Default|GetPlayerLocation) (Variables|Default|GetPlayerRotation) (Variables|Default|GetDialogueTreeIndex_Pink)))