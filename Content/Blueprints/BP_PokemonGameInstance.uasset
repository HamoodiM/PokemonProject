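; Game instance for a Pokémon-style game that holds persistent player state: party, starter, names, story flags, money and inventory.
; SaveGame writes this state, the player transform and NPC_Pink's dialogue index to one SG_PokemonSave slot; LoadGame restores instance variables and returns the save object.
; Healing rebuilds party structs with full HP and PP.
; Party (capped at six), money and stacked-item helpers fire change notifications.
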(fn SaveGame
  (bind _returnvalue (Game|Player|GetPlayerPawn 0))
  (bind _returnvalue_2 (SaveGame|CreateSaveGameObject "/Game/Blueprints/SG_PokemonSave.SG_PokemonSave_C"))
  (bind _assg_pokemon_save (Utilities|Casting|CastToSG_PokemonSave _returnvalue_2))
  (bind _returnvalue_3 (Actor|GetActorOfClass "/Game/Blueprints/Trainers/NPC_Pink.NPC_Pink_C"))
  (bind _asac_dialogue_pink (Utilities|Casting|CastToAC_Dialogue_Pink (Actor|GetComponentbyClass _returnvalue_3 "/Game/Blueprints/Dialogue/AC_Dialogue_Pink.AC_Dialogue_Pink_C")))
  (bind _dialoguetreeindex (Default|GetDialogueTreeIndex _asac_dialogue_pink))
  (Default|Populate _assg_pokemon_save (Variables|Default|GetbStarterChosen) (Variables|Default|GetParty) (Transformation|GetActorLocation _returnvalue) (Transformation|GetActorRotation _returnvalue) _dialoguetreeindex)
  (Default|PopulateStory _assg_pokemon_save (Variables|Default|GetPlayerName) (Variables|Default|GetRivalName) (Variables|Default|GetbIntroComplete) (Variables|Default|GetbRivalDefeated))
  (Default|PopulateItems _assg_pokemon_save (Variables|Default|GetMoney) (Variables|Default|GetInventory))
  (SaveGame|SaveGametoSlot _assg_pokemon_save "PlayerSave"))

(fn LoadGame
  (bind _returnvalue (SaveGame|DoesSaveGameExist "PlayerSave"))
  (if _returnvalue
    (bind _returnvalue_2 (SaveGame|LoadGamefromSlot "PlayerSave"))
    (bind _assg_pokemon_save (Utilities|Casting|CastToSG_PokemonSave _returnvalue_2)
      (:then
        (bind (_bstarterchosen _party) (Default|GetData _assg_pokemon_save))
        (Variables|Default|SetbStarterChosen _bstarterchosen)
        (Variables|Default|SetParty _party)
        (bind (_outplayername _outrivalname _outintrocomplete _outrivaldefeated) (Default|GetStoryData _assg_pokemon_save))
        (Variables|Default|SetPlayerName _outplayername)
        (Variables|Default|SetRivalName _outrivalname)
        (Variables|Default|SetbIntroComplete _outintrocomplete)
        (Variables|Default|SetbRivalDefeated _outrivaldefeated)
        (bind (_money _inventory) (Default|GetItemsData _assg_pokemon_save))
        (Variables|Default|SetMoney _money)
        (Variables|Default|SetInventory _inventory)
        (return true _assg_pokemon_save))
      (:CastFailed
        (return false _assg_pokemon_save)))
    (else
      (return false 0))))

(fn HealStats
  (params (InStats :type S%20Pokemon%20Stats%20Structure))
  (bind (_hp _maxhp _attack _maxattack _defence _maxdefence _spattack _maxspattack _spdefence _maxspdefence _speed _maxspeed) (Utilities|Struct|BreakS_PokemonStats InStats))
  (return (Utilities|Struct|MakeS_PokemonStats _maxhp _maxhp _attack _maxattack _defence _maxdefence _spattack _maxspattack _spdefence _maxspdefence _speed _maxspeed)))

(fn HealMove
  (params (InMove :type S%20TM%20Move%20Structure))
  (bind (_movename _movetype _moveaccuracy _movepower _ppcurrent _ppmax _levellearnt _movecategory _stattochange _statchangeamount _statchangetarget _statustoapply _statuschance _ismultihit _istwoturn _forcesswitch _iscountermove) (Utilities|Struct|BreakS_TMMove InMove))
  (return (Utilities|Struct|MakeS_TMMove _movename _movetype _moveaccuracy _movepower _ppmax _ppmax _levellearnt _movecategory _stattochange _statchangeamount _statchangetarget _statustoapply _statuschance _ismultihit _istwoturn _forcesswitch _iscountermove)))

(fn HealMember
  (params (InMember :type S%20Party%20Member%20Structure))
  (bind (_pokemon _stats _moves) (Utilities|Struct|BreakS_PartyMember InMember))
  (Utilities|Array|Clear (LocalVariables|GetHealedMoves))
  (for _index (range 0 (- (Utilities|Array|Length _moves) (Class|KismetSystemLibrary|MakeLiteralInteger 1)))
    (bind _outmove (CallFunction|HealMove (Utilities|Array|Get(acopy) _moves _index)))
    (Utilities|Array|Add (LocalVariables|GetHealedMoves) _outmove))
  (bind _outstats (CallFunction|HealStats _stats))
  (return (Utilities|Struct|MakeS_PartyMember _pokemon _outstats (LocalVariables|GetHealedMoves))))

(fn HealParty
  (Utilities|Array|Clear (LocalVariables|GetHealedParty))
  (for _index (range 0 (- (Utilities|Array|Length (Variables|Default|GetParty)) (Class|KismetSystemLibrary|MakeLiteralInteger 1)))
    (bind _outmember (CallFunction|HealMember (Utilities|Array|Get(acopy) (Variables|Default|GetParty) _index)))
    (Utilities|Array|Add (LocalVariables|GetHealedParty) _outmember))
  (Variables|Default|SetParty (LocalVariables|GetHealedParty))
  (Default|CallOnPartyChanged))

(fn AddMoney
  (params (Amount :type Integer))
  (Variables|Default|SetMoney (+ (Variables|Default|GetMoney) Amount))
  (Default|CallOnMoneyChanged)
  (return true))

(fn RemoveMoney
  (params (Amount :type Integer))
  (if (>= (Variables|Default|GetMoney) Amount)
    (Variables|Default|SetMoney (- (Variables|Default|GetMoney) Amount))
    (Default|CallOnMoneyChanged)
    (return true)
    (else
      (return false))))

(fn AddItem
  (params (ItemRow :type Name) (Quantity :type Integer))
  (bind _inventory (Variables|Default|GetInventory))
  (Variables|Default|SetbItemFound false)
  (for _index (range 0 (- (Utilities|Array|Length _inventory) (Class|KismetSystemLibrary|MakeLiteralInteger 1)))
    (if (== (.Item (Utilities|Struct|BreakS_ItemStack (Utilities|Array|Get(acopy) _inventory _index))) ItemRow)
      (Utilities|Array|SetArrayElem _inventory _index (Utilities|Struct|MakeS_ItemStack ItemRow (+ (.Quantity (Utilities|Struct|BreakS_ItemStack (Utilities|Array|Get(acopy) _inventory _index))) Quantity)))
      (Variables|Default|SetbItemFound true)))
  (if (not (Variables|Default|GetbItemFound))
    (Utilities|Array|Add _inventory (Utilities|Struct|MakeS_ItemStack ItemRow Quantity)))
  (Default|CallOnInventoryChanged))

(fn RemoveItem
  (params (ItemRow :type Name) (Quantity :type Integer))
  (bind _inventory (Variables|Default|GetInventory))
  (for _index (range 0 (- (Utilities|Array|Length _inventory) (Class|KismetSystemLibrary|MakeLiteralInteger 1)))
    (if (== (.Item (Utilities|Struct|BreakS_ItemStack (Utilities|Array|Get(acopy) _inventory _index))) ItemRow)
      (if (> Quantity (.Quantity (Utilities|Struct|BreakS_ItemStack (Utilities|Array|Get(acopy) _inventory _index))))
        (return false)
        (else
          (if (== Quantity (.Quantity (Utilities|Struct|BreakS_ItemStack (Utilities|Array|Get(acopy) _inventory _index))))
            (Utilities|Array|RemoveIndex _inventory _index)
            (else
              (Utilities|Array|SetArrayElem _inventory _index (Utilities|Struct|MakeS_ItemStack ItemRow (- (.Quantity (Utilities|Struct|BreakS_ItemStack (Utilities|Array|Get(acopy) _inventory _index))) Quantity)))))
          (Default|CallOnInventoryChanged)
          (return true)))))
  (return false))

(fn GetItemQuantity
  (params (ItemRow :type Name))
  (bind _inventory (Variables|Default|GetInventory))
  (for _index (range 0 (- (Utilities|Array|Length _inventory) (Class|KismetSystemLibrary|MakeLiteralInteger 1)))
    (if (== (.Item (Utilities|Struct|BreakS_ItemStack (Utilities|Array|Get(acopy) _inventory _index))) ItemRow)
      (return (.Quantity (Utilities|Struct|BreakS_ItemStack (Utilities|Array|Get(acopy) _inventory _index))))))
  (return 0))

(fn AddtoParty
  (params (Pokemon1 :type S%20Party%20Member%20Structure))
  (bind _party (Variables|Default|GetParty))
  (if (>= (Utilities|Array|Length _party) (Class|KismetSystemLibrary|MakeLiteralInteger 6))
    (return false)
    (else
      (Utilities|Array|Add _party Pokemon1)
      (Default|CallOnPartyChanged)
      (return true))))